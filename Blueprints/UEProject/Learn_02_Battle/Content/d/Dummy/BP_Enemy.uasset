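; Dummy enemy character with a sword, health bar and name label that reacts to player attacks and dies.
; AnyDamage runs chained macros: subtract StatusComponent health, face the attacker, flash red via dynamic materials, then die or react.
; Hit reactions branch on damage causer: sword and fist trigger the player's combo effect plus mass-scaled knockback, while wizard throws can briefly activate fire.
; Death disables capsule collision, plays a montage and destroys both actors; weapon getters/setters are stubs.
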(event `self.ReceiveBeginPlay`
  (`|ExecutionSequence`
    (:`then_0`
      (bind _returnvalue (`|SpawnActorFromClass` "/Game/Weapons/Combo/BP_Sword.BP_Sword_C" (`KismetMathLibrary.MakeTransform` (0.0 0.0 0.0)) "Undefined" "OverrideRootScale" self null))
      (set `self.Sword` _returnvalue)
      (`self.K2_AttachToComponent` (`self.Mesh`) "GreatSword" "KeepRelative" "KeepRelative" "KeepRelative"))
    (:`then_1`
      (`self.UpdateHealthBar`))
    (:`then_2`
      (bind _returnvalue_2 (`KismetMaterialLibrary.CreateDynamicMaterialInstance` "/Game/Materials/M_UE4Man_Body_Enemy.M_UE4Man_Body_Enemy"))
      (`KismetArrayLibrary.Array_Add` (`self.Materials`) _returnvalue_2)
      (bind _returnvalue_3 (`KismetMaterialLibrary.CreateDynamicMaterialInstance` "/Game/Materials/M_UE4Man_ChestLogo_Enemy.M_UE4Man_ChestLogo_Enemy"))
      (`KismetArrayLibrary.Array_Add` (`self.Materials`) _returnvalue_3)
      (`PrimitiveComponent.SetMaterial` (`self.Mesh`) 0 (`|GetArrayItem` (`self.Materials`)))
      (`PrimitiveComponent.SetMaterial` (`self.Mesh`) 1 (`|GetArrayItem` (`self.Materials`) 1)))
    (:`then_3`
      (`TextRenderComponent.K2_SetText` (`self.TextRender`) (`KismetTextLibrary.Conv_StringToText` (`KismetSystemLibrary.GetDisplayName` self))))
    (:`then_4`
      (`SceneComponent.SetVisibility` (`self.Cursor`) false false))))

(event `self.ReceiveAnyDamage`
  (params (Damage :type "Float (single-precision)") (DamageType :type "DamageType Object Reference") (InstigatedBy :type "Controller Object Reference") (DamageCauser :type "Actor Object Reference"))
  (set `self.Causer` DamageCauser)
  (bind _ascharacter (cast `Character` (`Controller.K2_GetPawn` InstigatedBy)))
  (set `self.Attacker` _ascharacter)
  (set `self.Damage` Damage)
  (set `/Game/Components/StatusComponent.Health` (- (`/Game/Components/StatusComponent.Health` (`self.StatusComponent`)) (`self.Damage`)) (`self.StatusComponent`))
  (`self.UpdateHealthBar`)
  (`self.K2_SetActorRotation` (`KismetMathLibrary.FindLookAtRotation` (`self.K2_GetActorLocation`) (`self.K2_GetActorLocation` (`self.Attacker`))))
  (`self.ChangeMaterial` (struct :`R` 1.0 :`A` 1.0))
  (`KismetSystemLibrary.Delay` 0.5)
  (`self.ChangeMaterial` (struct :`R` 0.45 :`G` 0.4 :`B` 0.36 :`A` 1.0))
  (if (<= (`/Game/Components/StatusComponent.Health` (`self.StatusComponent`)) 0.0)
    (`/Engine/EditorBlueprintResources/StandardMacros.DoOnce` false
      (:`Completed`
        (set `self.Dead` true)
        (`PrimitiveComponent.SetCollisionEnabled` (`self.CapsuleComponent`) "NoCollision")
        (bind _returnvalue (`self.PlayAnimMontage` "/Game/Character/Montages/DeadFall_Montage.DeadFall_Montage" 1.0 "Start"))
        (`KismetSystemLibrary.Delay` (- _returnvalue 2.0))
        (`self.K2_DestroyActor`)
        (`self.K2_DestroyActor` (`self.Sword`))))
    (else
      (`self.PlayAnimMontage` "/Game/Character/Montages/HitReaction_Montage.HitReaction_Montage" 3.0)
      (bind _asbp_combo (cast `/Game/Weapons/Combo/BP_Combo` (`self.Causer`))
        (:`then`
          (cast `/Game/Weapons/Combo/BP_Sword` (`self.Causer`)
            (:`then`
              (bind _asbp_player (cast `/Game/Player/BP_Player` (`self.Attacker`)))
              (`/Game/Player/BP_Player.PlayLastComboEffect` _asbp_player self (`/Game/Weapons/Combo/BP_Combo.LastEffect` _asbp_combo))
              (`self.K2_AddActorWorldOffset` (* (`KismetMathLibrary.Vector_Normal2D` (`self.GetActorForwardVector`)) (* (`CharacterMovementComponent.Mass` (`self.CharacterMovement`)) -0.2))))
            (:`CastFailed`
              (cast `/Game/Weapons/Combo/BP_Fist` (`self.Causer`))
              (bind _asbp_player_2 (cast `/Game/Player/BP_Player` (`self.Attacker`)))
              (`/Game/Player/BP_Player.PlayLastComboEffect` _asbp_player_2 self (`/Game/Weapons/Combo/BP_Combo.LastEffect` _asbp_combo))
              (`self.K2_AddActorWorldOffset` (* (`KismetMathLibrary.Vector_Normal2D` (`self.GetActorForwardVector`)) (* (`CharacterMovementComponent.Mass` (`self.CharacterMovement`)) -0.1))))))
        (:`CastFailed`
          (bind _asbp_wizard (cast `/Game/Weapons/Wizard/BP_Wizard` (`self.Causer`)))
          (bind _asbp_wizard_skill_throw (cast `/Game/Weapons/Wizard/BP_WizardSkill_Throw` (`/Game/Weapons/Wizard/BP_Wizard.Skill` _asbp_wizard)))
          (switch `int` (`/Game/Weapons/Wizard/BP_WizardSkill_Throw.Current` _asbp_wizard_skill_throw)
            (:`0`
              (`ActorComponent.SetActive` (`self.Fire`) true false)
              (`KismetSystemLibrary.Delay` 2.0)
              (`ActorComponent.SetActive` (`self.Fire`) false false))))))))

(fn `ChangeMaterial`
  (params (Color :type "LinearColor Structure"))
  (for _array_element (`self.Materials`)
    (`MaterialInstanceDynamic.SetVectorParameterValue` _array_element "BodyColor" (`local.Color`))))

(fn `GetWeapon_CanMove`
  (returns (CanMove :type Boolean))
  (return false))

(fn `GetWeapon_Combat`
  (returns (Combat :type "/Game/Enums/ECombatType Enum"))
  (return "NewEnumerator0"))

(fn `GetWeapon_Current`
  (returns (Weapon :type "/Game/Weapons/BP_Weapon Object Reference"))
  (return null))

(fn `GetWeapon_State`
  (returns (State :type "/Game/Enums/EStateType Enum"))
  (return "NewEnumerator0"))

(fn `SetWeapon_CanMove`
  (params (CanMove :type Boolean))
  (returns (Result :type Boolean))
  (return false))

(fn `SetWeapon_Combat`
  (params (Combat :type "/Game/Enums/ECombatType Enum" :default "NewEnumerator0"))
  (returns (Result :type "/Game/Enums/ECombatType Enum"))
  (return "NewEnumerator0"))

(fn `SetWeapon_State`
  (params (State :type "/Game/Enums/EStateType Enum" :default "NewEnumerator0"))
  (returns (Result :type "/Game/Enums/EStateType Enum"))
  (return "NewEnumerator0"))

(fn `UpdateHealthBar`
  (bind _statuscomponent (`self.StatusComponent`))
  (bind _aswb_health_bar (cast `/Game/Widgets/WB_HealthBar` (`WidgetComponent.GetUserWidgetObject` (`self.HealthBar`))))
  (`/Game/Widgets/WB_HealthBar.Update HealthBar` _aswb_health_bar (`/Game/Components/StatusComponent.Health` _statuscomponent) (`/Game/Components/StatusComponent.MaxHealth` _statuscomponent)))

(fn `UserConstructionScript`)

(fn `Weapon_Change`
  (params (NewWeapon :type "/Game/Weapons/BP_Weapon Object Reference"))
  (returns (Weapon :type "/Game/Weapons/BP_Weapon Object Reference"))
  (return null))

(fn `Weapon_DecreaseHealth`
  (params (Health :type "Float (double-precision)"))
  (returns (Result :type "Float (double-precision)"))
  (return 0.0))

(fn `Weapon_IncreaseHealth`
  (params (Health :type "Float (double-precision)"))
  (returns (Result :type "Float (double-precision)"))
  (return 0.0))