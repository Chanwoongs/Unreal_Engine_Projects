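; Debug demo Blueprint that visualizes the cross product between a player's forward vector and the direction to an enemy.
; Each Tick it draws arrows from the player for the vector to the enemy, the scaled forward vector and their cross product.
; It also prints the enemy location, the cross product and its dot with the player's up vector, a signed left/right indicator.
; Small helper functions read the Player and Enemy references.
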(event `self.ReceiveTick`
  (params (DeltaSeconds :type "Float (single-precision)"))
  (bind _returnvalue (`self.GetPlayerLocation`))
  (bind _returnvalue_2 (`self.GetPlayerLocation`))
  (bind _returnvalue_3 (`self.GetPlayerLocation`))
  (bind _returnvalue_4 (`KismetMathLibrary.Cross_VectorVector` (`self.GetPlayerForwardVector`) (`self.GetPlayerToEnemy`)))
  (`|ExecutionSequence`
    (:`then_0`
      (`KismetSystemLibrary.DrawDebugArrow` _returnvalue_2 (+ _returnvalue_2 (`self.GetPlayerToEnemy`)) 100.0 (struct :`R` 1.0 :`A` 1.0)))
    (:`then_1`
      (`KismetSystemLibrary.DrawDebugArrow` _returnvalue_3 (+ _returnvalue_3 (* (`self.GetPlayerForwardVector`) 300.0)) 100.0 (struct :`G` 1.0 :`B` 0.217642 :`A` 1.0)))
    (:`then_2`
      (`KismetSystemLibrary.DrawDebugArrow` _returnvalue (+ _returnvalue (`KismetMathLibrary.Cross_VectorVector` (`self.GetPlayerForwardVector`) (`self.GetPlayerToEnemy`))) 100.0 (struct :`G` 0.126143 :`B` 1.0 :`A` 1.0)))
    (:`then_3`
      (`KismetSystemLibrary.PrintString` (`KismetStringLibrary.Concat_StrStr` (`KismetStringLibrary.Conv_VectorToString` (`self.GetEnemyLocation`)) "/" (`KismetStringLibrary.Conv_VectorToString` _returnvalue_4) "/" (`KismetStringLibrary.Conv_DoubleToString` (`KismetMathLibrary.Dot_VectorVector` _returnvalue_4 (`self.GetPlayerUpVector`))))))))

(fn `GetEnemyLocation`
  (returns (ReturnValue :type "Vector Structure"))
  (return (`self.K2_GetActorLocation` (`self.Enemy`))))

(fn `GetPlayerForwardVector`
  (returns (ReturnValue :type "Vector Structure"))
  (return (`self.GetActorForwardVector` (`self.Player`))))

(fn `GetPlayerLocation`
  (returns (ReturnValue :type "Vector Structure"))
  (return (`self.K2_GetActorLocation` (`self.Player`))))

(fn `GetPlayerRotation`
  (returns (ReturnValue :type "Rotator Structure"))
  (return (`self.K2_GetActorRotation` (`self.Player`))))

(fn `GetPlayerToEnemy`
  (returns (ReturnValue :type "Vector Structure"))
  (return (- (`self.K2_GetActorLocation` (`self.Enemy`)) (`self.K2_GetActorLocation` (`self.Player`)))))

(fn `GetPlayerUpVector`
  (returns (ReturnValue :type "Vector Structure"))
  (return (`self.GetActorUpVector` (`self.Player`))))

(fn `UserConstructionScript`)