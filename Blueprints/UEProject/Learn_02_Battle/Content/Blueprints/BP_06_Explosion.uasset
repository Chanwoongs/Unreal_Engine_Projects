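; Explosion actor Blueprint whose Explosion event plays a fire effect and blasts nearby physics objects away.
; The event spawns the particle emitter at an offset from the actor, then runs a short upward multi-sphere trace for PhysicsBody objects, with debug drawing on.
; Each hit static mesh component receives a constant-falloff radial impulse from the actor's location, with strength scaled by the component's mass.
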(event `Explosion`
  (`GameplayStatics.SpawnEmitterAtLocation` "/Game/Explosion/Fire_Exp_03.Fire_Exp_03" (+ (`KismetMathLibrary.MakeVector` -250.0) (`self.K2_GetActorLocation`)))
  (bind _outhits (`KismetSystemLibrary.SphereTraceMultiForObjects` :`Start` (`self.K2_GetActorLocation`) :`End` (+ (`self.K2_GetActorLocation`) (`KismetMathLibrary.MakeVector` 0.0 0.0 100.0)) :`Radius` 300.0 :`ObjectTypes` (`|MakeArray` "ObjectTypeQuery4" :!type "EObjectTypeQuery Enum") :`DrawDebugType` "ForDuration" :`TraceColor` (struct :`G` 1.0 :`A` 1.0) :`TraceHitColor` (struct :`R` 1.0 :`A` 1.0) :`DrawTime` 10.0))
  (for _array_element _outhits
    (bind _asstatic_mesh_component (cast `StaticMeshComponent` (`.HitComponent` (`GameplayStatics.BreakHitResult` _array_element))))
    (`PrimitiveComponent.AddRadialImpulse` _asstatic_mesh_component (`self.K2_GetActorLocation`) 300.0 (* (`PrimitiveComponent.GetMass` _asstatic_mesh_component) 1000.0) "RIF_Constant" false)))

(fn `UserConstructionScript`)