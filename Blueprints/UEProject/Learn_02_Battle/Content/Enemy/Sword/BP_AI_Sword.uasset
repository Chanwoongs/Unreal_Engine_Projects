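; BP_AI_Sword is a sword-wielding enemy character Blueprint that arms itself with a great sword when play begins.
; After the parent BeginPlay, Spawn&AttachSword spawns a BP_GreatSword owned by the enemy and stores it in the GreatSword variable.
; The sword attaches to the GreatSword socket on the Mesh with relative transforms, and all other behavior is left to the parent class.
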(event `self.ReceiveBeginPlay`
  (`parent.ReceiveBeginPlay`)
  (bind _returnvalue (`|SpawnActorFromClass` "/Game/Weapons/Combo/BP_GreatSword.BP_GreatSword_C" (`KismetMathLibrary.MakeTransform` (0.0 0.0 0.0)) "Undefined" "OverrideRootScale" self null))
  (bind _output_get (set `self.GreatSword` _returnvalue))
  (`self.K2_AttachToComponent` _output_get (`self.Mesh`) "GreatSword" "KeepRelative" "KeepRelative" "KeepRelative" true))

(fn `UserConstructionScript`
  (`parent.UserConstructionScript`))