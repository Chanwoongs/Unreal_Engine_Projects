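; AI controller for BP_AI enemies that runs their behavior and tracks the player through perception.
; On possess, it runs the behavior tree assigned on the possessed BP_AI, if valid.
; On each perception update, it searches currently perceived actors for a BP_Player and writes the first match to the Player blackboard key, clearing the key when none is found.
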(event `self.ReceivePossess`
  (params (PossessedPawn :type "Pawn Object Reference"))
  (bind _asbp_ai (cast `/Game/Enemy/BP_AI` PossessedPawn))
  (bind _output_get (set `self.AICharacter` _asbp_ai))
  (bind _behaviortree (`/Game/Enemy/BP_AI.BehaviorTree` _output_get)
    (:`then`
      (`self.RunBehaviorTree` _behaviortree))
    (:`else`)))

(event `self.AIPerception.OnPerceptionUpdated`
  (params (UpdatedActors :type "Array of Actor Object Reference (by ref)"))
  (set `self.FoundPlayer` false)
  (for _array_element (`AIPerceptionComponent.GetCurrentlyPerceivedActors` (`self.AIPerception`) null) :!label _label
    (cast `/Game/Player/BP_Player` _array_element)
    (`BlackboardComponent.SetValueAsObject` (`AIBlueprintHelperLibrary.GetBlackboard` null) "Player" _array_element)
    (set `self.FoundPlayer` true)
    (`self.PerceivedActorsBreak`))
  (if (not (`self.FoundPlayer`))
    (`BlackboardComponent.SetValueAsObject` (`AIBlueprintHelperLibrary.GetBlackboard` null) "Player" null)))

(event `PerceivedActorsBreak`
  (goto _label :!via `Break`))

(fn `UserConstructionScript`)