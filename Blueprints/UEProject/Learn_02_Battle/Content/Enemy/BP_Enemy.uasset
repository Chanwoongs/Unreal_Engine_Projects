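; Enemy character that spawns with an attached sword, a health bar widget and dynamic body materials, and reacts to damage until it dies.
; Damage lowers health, turns it toward the attacker and flashes it red, then triggers the player's last combo effect.
; Survivors play a hit reaction with sword knockback or a temporary fireball burn.
; Death disables capsule collision, plays a montage, then destroys enemy and sword.
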(event `self.ReceiveBeginPlay`
  (`|ExecutionSequence`
    (:`then_0`
      (bind _returnvalue (`|SpawnActorFromClass` "/Game/Weapons/BP_Sword.BP_Sword_C" (`KismetMathLibrary.MakeTransform` (0.0 0.0 0.0)) "Undefined" "OverrideRootScale" self null))
      (bind _output_get (set `self.Sword` _returnvalue))
      (`self.K2_AttachToComponent` _output_get (`self.Mesh`) "GreatSword" "KeepRelative" "KeepRelative" "KeepRelative" true))
    (:`then_1`
      (`self.UpdateHealthBar`))
    (:`then_2`
      (bind _returnvalue_2 (`KismetMaterialLibrary.CreateDynamicMaterialInstance` "/Game/Materials/M_UE4Man_Body_Enemy.M_UE4Man_Body_Enemy"))
      (`KismetArrayLibrary.Array_Add` (`self.Materials`) _returnvalue_2)
      (bind _returnvalue_3 (`KismetMaterialLibrary.CreateDynamicMaterialInstance` "/Game/Materials/M_UE4Man_ChestLogo_Enemy.M_UE4Man_ChestLogo_Enemy"))
      (`KismetArrayLibrary.Array_Add` (`self.Materials`) _returnvalue_3)
      (`PrimitiveComponent.SetMaterial` (`self.Mesh`) 0 (`|GetArrayItem` (`self.Materials`)))
      (`PrimitiveComponent.SetMaterial` (`self.Mesh`) 1 (`|GetArrayItem` (`self.Materials`) 1)))))

(event `self.ReceiveAnyDamage`
  (params (Damage :type "Float (single-precision)") (DamageType :type "DamageType Object Reference") (InstigatedBy :type "Controller Object Reference") (DamageCauser :type "Actor Object Reference"))
  (set `self.Causer` DamageCauser)
  (bind _ascharacter (cast `Character` (`Controller.K2_GetPawn` InstigatedBy)))
  (set `self.Attacker` _ascharacter)
  (set `self.Damage` Damage)
  (set `self.Health` (- (`self.Health`) (`self.Damage`)))
  (`self.UpdateHealthBar`)
  (`self.K2_SetActorRotation` (`KismetMathLibrary.FindLookAtRotation` (`self.K2_GetActorLocation`) (`self.K2_GetActorLocation` (`self.Attacker`))))
  (`self.ChangeMaterial` (struct :`R` 1.0 :`A` 1.0))
  (`KismetSystemLibrary.Delay` 0.5)
  (`self.ChangeMaterial` (struct :`R` 0.45 :`G` 0.4 :`B` 0.36 :`A` 1.0))
  (bind _asbp_player (cast `/Game/Player/BP_Player` (`self.Attacker`)))
  (`/Game/Player/BP_Player.PlayLastComboEffect` _asbp_player self)
  (if (<= (`self.Health`) 0.0)
    (`/Engine/EditorBlueprintResources/StandardMacros.DoOnce` false
      (:`Completed`
        (set `self.Dead` true)
        (`PrimitiveComponent.SetCollisionEnabled` (`self.CapsuleComponent`) "NoCollision")
        (bind _returnvalue (`self.PlayAnimMontage` "/Game/Character/Montages/DeadFall_Montage.DeadFall_Montage" 1.0 "Start"))
        (`KismetSystemLibrary.Delay` (- _returnvalue 2.0))
        (`self.K2_DestroyActor`)
        (`self.K2_DestroyActor` (`self.Sword`))))
    (else
      (`self.PlayAnimMontage` "/Game/Character/Montages/HitReaction_Montage.HitReaction_Montage" 3.0)
      (cast `/Game/Weapons/BP_Sword` (`self.Causer`)
        (:`then`
          (`self.K2_AddActorWorldOffset` (* (`KismetMathLibrary.Vector_Normal2D` (`self.GetActorForwardVector`)) (* (`CharacterMovementComponent.Mass` (`self.CharacterMovement`)) -0.2))))
        (:`CastFailed`
          (cast `/Game/Weapons/BP_FireBall` (`self.Causer`))
          (`ActorComponent.SetActive` (`self.Fire`) true false)
          (`KismetSystemLibrary.Delay` 2.0)
          (`ActorComponent.SetActive` (`self.Fire`) false false))))))

(fn `ChangeMaterial`
  (params (Color :type "LinearColor Structure"))
  (for _array_element (`self.Materials`)
    (`MaterialInstanceDynamic.SetVectorParameterValue` _array_element "BodyColor" (`local.Color`))))

(fn `UpdateHealthBar`
  (bind _aswb_health_bar (cast `/Game/Enemy/WB_HealthBar` (`WidgetComponent.GetUserWidgetObject` (`self.HealthBar`))))
  (`/Game/Enemy/WB_HealthBar.Update HealthBar` _aswb_health_bar (`self.Health`)))

(fn `UserConstructionScript`)