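; BP_AI_Sword is a child enemy AI Blueprint that fights with a greatsword.
; On BeginPlay it spawns a BP_GreatSword it owns and attaches it to the holster socket on its mesh.
; Overrides of the parent's grab and ungrab events move the sword between the hand and holster sockets.
; Equipped and UnEquipped extend the parent logic, calling WeaponChange and switching the Combat enum state.
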(event `self.ReceiveBeginPlay`
  (`parent.ReceiveBeginPlay`)
  (bind _returnvalue (`|SpawnActorFromClass` "/Game/Weapons/Combo/BP_GreatSword.BP_GreatSword_C" (`KismetMathLibrary.MakeTransform` (0.0 0.0 0.0)) "Undefined" "OverrideRootScale" self null))
  (bind _output_get (set `self.GreatSword` _returnvalue))
  (`self.K2_AttachToComponent` _output_get (`self.Mesh`) "Holster_GreatSword" "KeepRelative" "KeepRelative" "KeepRelative" true))

(event `self.GrabSword`
  (`parent.GrabSword`)
  (`self.K2_AttachToComponent` (`self.GreatSword`) (`self.Mesh`) "GreatSword" "KeepRelative" "KeepRelative" "KeepRelative" true))

(event `self.UnGrabSword`
  (`parent.UnGrabSword`)
  (`self.K2_AttachToComponent` (`self.GreatSword`) (`self.Mesh`) "Holster_GreatSword" "KeepRelative" "KeepRelative" "KeepRelative" true))

(event `self.Equipped`
  (`parent.Equipped`)
  (`self.Weapon_Change` (`self.GreatSword`))
  (set `self.Combat` "NewEnumerator1"))

(event `self.UnEquipped`
  (`parent.UnEquipped`)
  (`self.Weapon_Change` null)
  (set `self.Combat` "NewEnumerator0"))

(fn `UserConstructionScript`
  (`parent.UserConstructionScript`))