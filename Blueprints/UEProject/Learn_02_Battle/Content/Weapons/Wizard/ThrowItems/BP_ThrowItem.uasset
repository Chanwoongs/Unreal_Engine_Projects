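; BP_ThrowItem is a Wizard throwable that deals damage to actors it hits and has a two-second lifespan.
; It resolves its owner chain through BP_WizardSkill_Throw to BP_Wizard.
; The BeginOverlap function copies its Power to the wizard and delegates damage to the wizard's SendDamage.
; On success, it spawns the supplied explosion at an offset from the target and destroys itself.
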(event `self.ReceiveBeginPlay`
  (`self.SetLifeSpan` 2.0))

(fn `BeginOverlap`
  (params (OtherActor :type "Actor Object Reference") (Explosion :type "ParticleSystem Object Reference") (Location :type "Vector Structure") (Scale :type "Vector Structure") (Rotation :type "Rotator Structure"))
  (bind _wizard (`self.GetOwnerToWizard`))
  (set `/Game/Weapons/BP_Weapon.Power` (`self.Power`) _wizard)
  (bind _result (`/Game/Weapons/BP_Weapon.SendDamage` _wizard (`local.OtherActor`)))
  (if _result
    (`GameplayStatics.SpawnEmitterAtLocation` (`local.Explosion`) (+ (`self.K2_GetActorLocation` (`local.OtherActor`)) (`local.Location`)) (`local.Rotation`) (`local.Scale`))
    (`self.K2_DestroyActor` self)))

(fn `GetOwnerToThrow`
  (returns (Throw :type "/Game/Weapons/Wizard/BP_WizardSkill_Throw Object Reference"))
  (bind _asbp_wizard_skill_throw (cast `/Game/Weapons/Wizard/BP_WizardSkill_Throw` (`self.GetOwner`)))
  (return _asbp_wizard_skill_throw))

(fn `GetOwnerToWizard`
  (returns (Wizard :type "/Game/Weapons/Wizard/BP_Wizard Object Reference"))
  (bind _asbp_wizard (cast `/Game/Weapons/Wizard/BP_Wizard` (`self.GetOwner` (`self.GetOwnerToThrow`))))
  (return _asbp_wizard))

(fn `UserConstructionScript`)