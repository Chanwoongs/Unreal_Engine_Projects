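; Wizard warp skill that teleports the owning character to a cursor-picked point on an actor named "Wall".
; While this is the active skill, Tick traces WorldStatic under the cursor and moves a targeting decal to valid hits.
; Spell stores the hit location, locks movement and plays the warp montage, or resets wizard state on invalid targets.
; EndSpell restores movement and teleports the character to the stored location.
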(event `self.ReceiveBeginPlay`
  (`SceneComponent.SetVisibility` (`self.Decal`) false false))

(event `self.OnFocus`
  (`SceneComponent.SetVisibility` (`self.Decal`) true false))

(event `OffFocus`
  (`SceneComponent.SetVisibility` (`self.Decal`) false false))

(event `self.ReceiveTick`
  (params (DeltaSeconds :type "Float (single-precision)"))
  (bind _decal (`self.Decal`))
  (bind (_location _hitactor) (`self.GetCursorLocation`)
    (:`True`
      (if (== (`/Game/Weapons/Wizard/BP_Wizard.Skill` (`self.GetOwnerToWizard`)) self)
        (if (`KismetStringLibrary.EqualEqual_StrStr` (`KismetSystemLibrary.GetDisplayName` _hitactor) "Wall")
          (`SceneComponent.SetVisibility` _decal true false)
          (`SceneComponent.K2_SetWorldLocation` _decal _location false false)
          (else
            (`SceneComponent.SetVisibility` _decal false false :!label _label)))))
    (:`False`
      (goto _label))))

(event `self.Spell`
  (bind (_location _hitactor) (`self.GetCursorLocation`)
    (:`True`
      (if (`KismetStringLibrary.EqualEqual_StrStr` (`KismetSystemLibrary.GetDisplayName` _hitactor) "Wall")
        (`self.K2_SetActorLocation` _location)
        (`/Game/Weapons/BP_Weapon.SetCanMove` (`self.GetOwnerToWizard`) false)
        (set `self.Location` _location)
        (bind _ascharacter (cast `Character` (`self.GetOwner` (`self.GetOwnerToWizard`))))
        (`Character.PlayAnimMontage` _ascharacter "/Game/Character/Montages/Wizard_Warp.Wizard_Warp" 1.5 "None")
        (else
          (`/Game/Weapons/BP_Weapon.SetCanMove` (`self.GetOwnerToWizard`) true :!label _label_2)
          (`/Game/Weapons/BP_Weapon.SetState` (`self.GetOwnerToWizard`) "NewEnumerator0"))))
    (:`False`
      (goto _label_2))))

(event `self.EndSpell`
  (`/Game/Weapons/BP_Weapon.SetCanMove` (`self.GetOwnerToWizard`) true)
  (`self.K2_SetActorLocation` (`self.GetOwner` (`self.GetOwnerToWizard`)) (`self.Location`) false true))

(fn `UserConstructionScript`
  (`parent.UserConstructionScript`))