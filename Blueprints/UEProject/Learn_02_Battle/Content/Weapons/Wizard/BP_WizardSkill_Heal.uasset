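; Wizard heal skill that handles the casting animation and movement lock for the spell.
; Spell disables movement through the owning wizard object, then plays the Wizard_Heal montage on that object's owning Character.
; EndSpell re-enables movement and is not triggered within this Blueprint.
; No healing is applied in this graph.
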(event `self.Spell`
  (`/Game/Weapons/BP_Weapon.SetCanMove` (`self.GetOwnerToWizard`) false)
  (bind _ascharacter (cast `Character` (`self.GetOwner` (`self.GetOwnerToWizard`))))
  (`Character.PlayAnimMontage` _ascharacter "/Game/Character/Montages/Wizard_Heal.Wizard_Heal" 1.0 "None"))

(event `self.EndSpell`
  (`/Game/Weapons/BP_Weapon.SetCanMove` (`self.GetOwnerToWizard`) true))

(fn `UserConstructionScript`
  (`parent.UserConstructionScript`))