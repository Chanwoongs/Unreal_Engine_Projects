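; Wizard weapon Blueprint that casts one of three skill actors: Heal, Warp or Throw.
; On BeginPlay it spawns the skills, attaches them to the owning character's mesh (Throw at a hand socket) and selects Heal.
; ChangeSkill swaps the active skill, moving focus from old to new, and weapon selection also toggles that focus.
; Attack and EndAttack delegate to the active skill's Spell and EndSpell.
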(event `OnSelected`
  (`/Engine/EditorBlueprintResources/StandardMacros.IsValid` (`self.Skill`)
    (:`Is Valid`
      (`/Game/Weapons/Wizard/BP_WizardSkill.OnFocus` (`self.Skill`)))))

(event `OffSelected`
  (`/Engine/EditorBlueprintResources/StandardMacros.IsValid` (`self.Skill`)
    (:`Is Valid`
      (`/Game/Weapons/Wizard/BP_WizardSkill.OffFocus` (`self.Skill`)))))

(event `self.ReceiveBeginPlay`
  (set `self.CombatType` "NewEnumerator2")
  (`|ExecutionSequence`
    (:`then_0`
      (bind _returnvalue (`|SpawnActorFromClass` "/Game/Weapons/Wizard/BP_WizardSkill_Heal.BP_WizardSkill_Heal_C" (`KismetMathLibrary.MakeTransform` (0.0 0.0 0.0)) "Undefined" "OverrideRootScale" self null))
      (set `self.Heal` _returnvalue)
      (bind _ascharacter (cast `Character` (`self.GetOwner`)))
      (`self.K2_AttachToComponent` (`self.Heal`) (`Character.Mesh` _ascharacter) "None" "KeepRelative" "KeepRelative" "KeepRelative" true))
    (:`then_1`
      (bind _returnvalue_2 (`|SpawnActorFromClass` "/Game/Weapons/Wizard/BP_WizardSkill_Warp.BP_WizardSkill_Warp_C" (`KismetMathLibrary.MakeTransform` (0.0 0.0 0.0)) "Undefined" "OverrideRootScale" self null))
      (set `self.Warp` _returnvalue_2)
      (bind _ascharacter_2 (cast `Character` (`self.GetOwner`)))
      (`self.K2_AttachToComponent` (`self.Warp`) (`Character.Mesh` _ascharacter_2) "None" "KeepRelative" "KeepRelative" "KeepRelative" true))
    (:`then_2`
      (bind _returnvalue_3 (`|SpawnActorFromClass` "/Game/Weapons/Wizard/BP_WizardSkill_Throw.BP_WizardSkill_Throw_C" (`KismetMathLibrary.MakeTransform` (0.0 0.0 0.0)) "Undefined" "OverrideRootScale" self null))
      (set `self.Throw` _returnvalue_3)
      (bind _ascharacter_3 (cast `Character` (`self.GetOwner`)))
      (`self.K2_AttachToComponent` (`self.Throw`) (`Character.Mesh` _ascharacter_3) "HandFireBall" "KeepRelative" "KeepRelative" "KeepRelative" true))
    (:`then_3`
      (`self.ChangeSkill` (`self.Heal`)))))

(event `self.Attack`
  (if (and (`self.CanAttack`) (`KismetSystemLibrary.IsValid` (`self.Skill`)))
    (`self.SetState` "NewEnumerator4")
    (`/Game/Weapons/Wizard/BP_WizardSkill.Spell` (`self.Skill`))))

(event `self.EndAttack`
  (`parent.EndAttack`)
  (`/Game/Weapons/Wizard/BP_WizardSkill.EndSpell` (`self.Skill`)))

(fn `ChangeSkill`
  (params (NewSkill :type "/Game/Weapons/Wizard/BP_WizardSkill Object Reference"))
  (returns (Weapon :type "/Game/Weapons/BP_Weapon Object Reference") (Skill :type "/Game/Weapons/Wizard/BP_WizardSkill Object Reference"))
  (bind _newskill (`local.NewSkill`))
  (if (!= NewSkill (`self.Skill`))
    (`/Engine/EditorBlueprintResources/StandardMacros.IsValid` (`self.Skill`)
      (:`Is Valid`
        (`/Game/Weapons/Wizard/BP_WizardSkill.OffFocus` (`self.Skill`)))
      (:`Is Not Valid`
        _))
    (`/Engine/EditorBlueprintResources/StandardMacros.IsValid` (`local.NewSkill`)
      (:`Is Valid`
        (bind _output_get (set `self.Skill` _newskill))
        (`/Game/Weapons/Wizard/BP_WizardSkill.OnFocus` _output_get)
        (return null _newskill))
      (:`Is Not Valid`
        (set `self.Skill` null)))))

(fn `UserConstructionScript`)