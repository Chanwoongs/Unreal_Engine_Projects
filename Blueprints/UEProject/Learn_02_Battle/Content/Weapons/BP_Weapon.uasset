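; BP_Weapon is a base weapon Blueprint with empty selection, Attack and EndAttack hooks for specific weapons to fill in.
; It reads and changes the owner's state, combat type, movement permission and health through BP_IWeapon interface messages, avoiding a hard cast to the owner.
; CanAttack checks that combat type matches and state is the first enum value.
; SendDamage applies Power as damage to any Character other than the owner.
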(event `OnSelected`)

(event `OffSeclected`)

(fn `Attack`)

(fn `CanAttack`
  (returns (Result :type Boolean))
  (return (and (`|EnumEquality` (`self.CombatType`) (`self.GetCombat`)) (`|EnumEquality` (`self.GetState`) "NewEnumerator0"))))

(fn `DecreaseHealth`
  (params (Health :type "Float (double-precision)"))
  (returns (Result :type "Float (double-precision)"))
  (bind _returnvalue (`self.GetOwner`))
  (if (`KismetSystemLibrary.DoesImplementInterface` _returnvalue "/Game/BP_IWeapon.BP_IWeapon_C")
    (bind _result (message `/Game/BP_IWeapon.Weapon_DecreaseHealth` _returnvalue Health))
    (return _result)))

(fn `EndAttack`)

(fn `GetCanMove`
  (returns (CanMove :type Boolean))
  (bind _returnvalue (`self.GetOwner`))
  (if (`KismetSystemLibrary.DoesImplementInterface` _returnvalue "/Game/BP_IWeapon.BP_IWeapon_C")
    (bind _canmove (message `/Game/BP_IWeapon.GetWeapon_CanMove` _returnvalue))
    (return _canmove)))

(fn `GetCombat`
  (returns (Combat :type "/Game/Enums/ECombatType Enum"))
  (bind _returnvalue (`self.GetOwner`))
  (if (`KismetSystemLibrary.DoesImplementInterface` _returnvalue "/Game/BP_IWeapon.BP_IWeapon_C")
    (bind _combat (message `/Game/BP_IWeapon.GetWeapon_Combat` _returnvalue))
    (return _combat)))

(fn `GetState`
  (returns (State :type "/Game/Enums/EStateType Enum"))
  (bind _returnvalue (`self.GetOwner`))
  (if (`KismetSystemLibrary.DoesImplementInterface` _returnvalue "/Game/BP_IWeapon.BP_IWeapon_C")
    (bind _state (message `/Game/BP_IWeapon.GetWeapon_State` _returnvalue))
    (return _state)))

(fn `IncreaseHealth`
  (params (Health :type "Float (double-precision)"))
  (returns (Result :type "Float (double-precision)"))
  (bind _returnvalue (`self.GetOwner`))
  (if (`KismetSystemLibrary.DoesImplementInterface` _returnvalue "/Game/BP_IWeapon.BP_IWeapon_C")
    (bind _result (message `/Game/BP_IWeapon.Weapon_IncreaseHealth` _returnvalue Health))
    (return _result)))

(fn `SendDamage`
  (params (OtherActor :type "Actor Object Reference"))
  (returns (Result :type Boolean))
  (if (!= (`self.GetOwner`) OtherActor)
    (bind _ascharacter (cast `Character` OtherActor)
      (:`then`
        (`GameplayStatics.ApplyDamage` _ascharacter (`self.Power`) (`self.GetInstigatorController` (`self.GetOwner`)) self)
        (return true))
      (:`CastFailed`
        (return false)))
    (else
      (return false))))

(fn `SetCanMove`
  (params (CanMove :type Boolean))
  (bind _returnvalue (`self.GetOwner`))
  (if (`KismetSystemLibrary.DoesImplementInterface` _returnvalue "/Game/BP_IWeapon.BP_IWeapon_C")
    (message `/Game/BP_IWeapon.SetWeapon_CanMove` _returnvalue CanMove)))

(fn `SetCombat`
  (params (Combat :type "/Game/Enums/ECombatType Enum" :default "NewEnumerator0"))
  (bind _returnvalue (`self.GetOwner`))
  (if (`KismetSystemLibrary.DoesImplementInterface` _returnvalue "/Game/BP_IWeapon.BP_IWeapon_C")
    (message `/Game/BP_IWeapon.SetWeapon_Combat` _returnvalue Combat)
    (return)))

(fn `SetState`
  (params (State :type "/Game/Enums/EStateType Enum" :default "NewEnumerator0"))
  (bind _returnvalue (`self.GetOwner`))
  (if (`KismetSystemLibrary.DoesImplementInterface` _returnvalue "/Game/BP_IWeapon.BP_IWeapon_C")
    (message `/Game/BP_IWeapon.SetWeapon_State` _returnvalue State)
    (return)))

(fn `UserConstructionScript`)