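; BP_Sword is a combo-system melee weapon Blueprint that deals damage to actors overlapping its capsule hitbox.
; The capsule's collision starts disabled at BeginPlay and is switched on and off through OnCollision and OffCollision.
; Each overlap passes the other actor to SendDamage, which is not defined in this Blueprint.
; Selection and deselection events only print debug strings.
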(event `self.ReceiveBeginPlay`
  (`self.OffCollision`)
  (`parent.ReceiveBeginPlay`))

(event `self.Capsule.OnComponentBeginOverlap`
  (params (OverlappedComponent :type "PrimitiveComponent Object Reference") (OtherActor :type "Actor Object Reference") (OtherComp :type "PrimitiveComponent Object Reference") (OtherBodyIndex :type Integer) (bFromSweep :type Boolean) (SweepResult :type "HitResult Structure (by ref)"))
  (`self.SendDamage` OtherActor))

(event `self.OnCollision`
  (`PrimitiveComponent.SetCollisionEnabled` (`self.Capsule`) "QueryAndPhysics"))

(event `self.OffCollision`
  (`PrimitiveComponent.SetCollisionEnabled` (`self.Capsule`) "NoCollision"))

(event `self.OnSelected`
  (`KismetSystemLibrary.PrintString` "Sword"))

(event `self.OffSeclected`
  (`KismetSystemLibrary.PrintString` "!Sword"))

(fn `UserConstructionScript`)