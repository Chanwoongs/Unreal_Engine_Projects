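; BP_Combo is a combo attack weapon that plays chained montages on its owning Character.
; BeginPlay fills the montage list from ComboTable rows, each defining montage, play rate, start section and movement permission.
; Attack starts the combo, or queues the next step when EnableNextCombo is open.
; PlayNextCombo plays queued steps and flags the last, EndAttack resets state and movement, and collision events are empty.
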(event `self.ReceiveBeginPlay`
  (bind _combotable (`self.ComboTable`))
  ;[1 1 1] Begin Play
  (bind _outrownames (`DataTableFunctionLibrary.GetDataTableRowNames` _combotable))
  (for _array_element _outrownames
    (bind _returnvalue (`|GetDataTableRow` _combotable _array_element)
      (:`then`
        (`KismetArrayLibrary.Array_Add` (`self.ComboMontages`) _returnvalue)))))

(event `self.Attack`
  ;[1 1 1] Attack
  (if (`self.EnableNextCombo`)
    (`/Engine/EditorBlueprintResources/StandardMacros.IncrementInt` (`self.ComboCount`)
      (:`  `
        (set `self.ExistNextCombo` true)
        (set `self.EnableNextCombo` false)))
    (elif (`self.CanAttack`)
      (`self.SetState` "NewEnumerator1")
      (`self.PlayComboMontage`))))

(event `PlayNextCombo`
  ;[1 1 1] Play Next Combo
  (if (`self.ExistNextCombo`)
    (`self.PlayComboMontage`)
    (set `self.ExistNextCombo` false)
    (set `self.LastCombo` (== (- (`KismetArrayLibrary.Array_Length` (`self.ComboMontages`)) 1) (`self.ComboCount`)))))

(event `self.EndAttack`
  ;[1 1 1] End Attack
  (`self.SetState` "NewEnumerator0")
  (`self.SetCanMove` true)
  (set `self.ComboCount` 0)
  (set `self.ExistNextCombo` false)
  (set `self.LastCombo` false))

(event `OnCollision`)

(event `OffCollision`)

(fn `PlayComboMontage`
  (bind (_output_montage _output_playrate _output_startsectionname _output_canmove) (break `/Game/Weapons/FComboMontage` (`|GetArrayItem` (`self.ComboMontages`) (`self.ComboCount`))))
  (bind _ascharacter (cast `Character` (`self.GetOwner`)))
  (`Character.PlayAnimMontage` _ascharacter _output_montage _output_playrate _output_startsectionname)
  (`self.SetCanMove` _output_canmove))

(fn `UserConstructionScript`
  (`parent.UserConstructionScript`))